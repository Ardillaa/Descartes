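; Descartes is a controllable pawn with simple planar movement and a toggleable Doubting state.
; Each tick it combines the HMoving and VMoving values into a length-clamped vector, scales it by Speed and delta time, and feeds it to AddMovementInput.
; Releasing C calls SetDoubt, which flips Doubting and prints the new value; nothing else here uses that state.
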(event `Key|C`
  (params (Key :type "Key Structure"))
  (:`Released`
    (`self.SetDoubt` (`self.Doubting?`))))

(event `self.ReceiveTick`
  (params (DeltaSeconds :type "Float (single-precision)"))
  (`self.AddMovementInput` (* (`KismetMathLibrary.ClampVectorSize` (`KismetMathLibrary.MakeVector` (`self.GetInputAxisValue`) (`self.GetInputAxisValue`)) 0.0 1.0) (* DeltaSeconds (`self.Speed`)))))

(fn `SetDoubt`
  (params (`Doubting?` :type Boolean))
  (if `Doubting?`
    (bind _output_get (set `self.Doubting?` false))
    (`KismetSystemLibrary.PrintString` (`KismetStringLibrary.Conv_BoolToString` _output_get))
    (else
      (bind _output_get_2 (set `self.Doubting?` true))
      (`KismetSystemLibrary.PrintString` (`KismetStringLibrary.Conv_BoolToString` _output_get_2)))))

(fn `UserConstructionScript`)