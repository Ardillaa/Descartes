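; Pushable chest actor (a copy, by its name) that the Descartes player character nudges along local X or Y.
; Four side triggers each check the player's HMovement (X sides) or VMovement (Y sides) on begin overlap, then offset the actor along that side's fixed direction.
; Each overlap applies a single unswept step of Speed times delta time, without continuous movement or a check of which actor overlapped.
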(event `self.YRight.OnComponentBeginOverlap`
  (params (OverlappedComponent :type "PrimitiveComponent Object Reference") (OtherActor :type "Actor Object Reference") (OtherComp :type "PrimitiveComponent Object Reference") (OtherBodyIndex :type Integer) (bFromSweep :type Boolean) (SweepResult :type "HitResult Structure (by ref)"))
  (bind _asdescartes (cast `/Game/Blueprints/Descartes` (`GameplayStatics.GetPlayerCharacter` 0)))
  (if (!= (`/Game/Blueprints/Descartes.VMovement` _asdescartes) 0.0)
    (`self.K2_AddActorLocalOffset` (* (`KismetMathLibrary.ClampVectorSize` (`KismetMathLibrary.MakeVector` 0.0 1.0) 0.0 1.0) (* (`GameplayStatics.GetWorldDeltaSeconds`) (`self.Speed`))))))

(event `self.XFront.OnComponentBeginOverlap`
  (params (OverlappedComponent :type "PrimitiveComponent Object Reference") (OtherActor :type "Actor Object Reference") (OtherComp :type "PrimitiveComponent Object Reference") (OtherBodyIndex :type Integer) (bFromSweep :type Boolean) (SweepResult :type "HitResult Structure (by ref)"))
  ;[1 1 1] Empujar X
  (bind _asdescartes (cast `/Game/Blueprints/Descartes` (`GameplayStatics.GetPlayerCharacter` 0)))
  (if (!= (`/Game/Blueprints/Descartes.HMovement` _asdescartes) 0.0)
    (`self.K2_AddActorLocalOffset` (* (`KismetMathLibrary.ClampVectorSize` (`KismetMathLibrary.MakeVector` -1.0) 0.0 1.0) (* (`GameplayStatics.GetWorldDeltaSeconds`) (`self.Speed`))))))

(event `self.XBack.OnComponentBeginOverlap`
  (params (OverlappedComponent :type "PrimitiveComponent Object Reference") (OtherActor :type "Actor Object Reference") (OtherComp :type "PrimitiveComponent Object Reference") (OtherBodyIndex :type Integer) (bFromSweep :type Boolean) (SweepResult :type "HitResult Structure (by ref)"))
  ;[1 1 1] Empujar X
  (bind _asdescartes (cast `/Game/Blueprints/Descartes` (`GameplayStatics.GetPlayerCharacter` 0)))
  (if (!= (`/Game/Blueprints/Descartes.HMovement` _asdescartes) 0.0)
    (`self.K2_AddActorLocalOffset` (* (`KismetMathLibrary.ClampVectorSize` (`KismetMathLibrary.MakeVector` 1.0) 0.0 1.0) (* (`GameplayStatics.GetWorldDeltaSeconds`) (`self.Speed`))))))

(event `self.YLeft.OnComponentBeginOverlap`
  (params (OverlappedComponent :type "PrimitiveComponent Object Reference") (OtherActor :type "Actor Object Reference") (OtherComp :type "PrimitiveComponent Object Reference") (OtherBodyIndex :type Integer) (bFromSweep :type Boolean) (SweepResult :type "HitResult Structure (by ref)"))
  (bind _asdescartes (cast `/Game/Blueprints/Descartes` (`GameplayStatics.GetPlayerCharacter` 0)))
  (if (!= (`/Game/Blueprints/Descartes.VMovement` _asdescartes) 0.0)
    (`self.K2_AddActorLocalOffset` (* (`KismetMathLibrary.ClampVectorSize` (`KismetMathLibrary.MakeVector` 0.0 -1.0) 0.0 1.0) (* (`GameplayStatics.GetWorldDeltaSeconds`) (`self.Speed`))))))

(fn `UserConstructionScript`)